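; Base enemy that roams around its spawn point until given a player target, then faces, optionally taunts, chases and attacks it.
; A move-then-attack loop picks light, heavy, special or ranged attacks by distance and chance, waiting out random montages.
; Melee sphere and forward sphere-overlap hits apply per-type damage on authority; montages multicast and taunt sound plays via RepNotify.
; ClearTarget and DoRangeAttack are empty stubs.
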(event `self.ReceiveBeginPlay`
  ;[1 1 1] BeginPlay
  (`self.f_MovementState` "NewEnumerator1")
  (set `self.StaringLocation` (`self.K2_GetActorLocation`))
  (`KismetSystemLibrary.Delay` 1.0)
  (`self.SetRoaming`))

(event `self.SetRoaming`
  ;[1 1 1] Roaming
  (if (and (not (`self.isCombat`)) (not (`self.isRoaming`)))
    (`|AIMoveTo` self (`NavigationSystemV1.K2_GetRandomReachablePointInRadius` (`self.StaringLocation`) 1000.0 null null) null 70.0
      (:`then`
        (set `self.isRoaming` true))
      (:`OnSuccess`
        (set `self.isRoaming` false)
        (`KismetSystemLibrary.Delay` 5.0)
        (`self.SetRoaming`))
      (:`OnFail`
        (`self.ClearTarget`)))))

(event `self.SetPlayerTarget`
  (params (Target :type "Actor Object Reference"))
  ;[1 1 1] SetTarget
  (set `self.PlayerTarget` Target)
  (set `self.isCombat` true)
  (`self.SetActorTickEnabled` true)
  (set `self.StartCombatLocation` (`self.K2_GetActorLocation`))
  (`self.f_MovementState` "NewEnumerator2")
  (`self.CheckForTaunt`))

(event `self.ReceiveTick`
  (params (DeltaSeconds :type "Float (single-precision)"))
  (bind (_returnvalue_roll _returnvalue_pitch _returnvalue_yaw) (`KismetMathLibrary.BreakRotator` (`KismetMathLibrary.FindLookAtRotation` (`self.K2_GetActorLocation`) (`self.K2_GetActorLocation` (`self.PlayerTarget`)))))
  ;[1 1 1] SetTarget
  (if (`self.isCombat`)
    (`self.PlayerTarget`
      (:`then`
        (`self.K2_SetActorRotation` (`KismetMathLibrary.MakeRotator` 0.0 0.0 _returnvalue_yaw)))
      (:`else`))))

(event `self.CheckForTaunt`
  (bind _output (`self.f_GetMontage` (`self.TauntMontague`)))
  ;[1 1 1] Aggro
  (`Controller.StopMovement` (`self.GetController`))
  (if (>= (`self.GetDistanceTo` self (`self.PlayerTarget`)) 800.0)
    (set `self.isTaunt` true)
    (`self.Multi_PlayerMontague` (`self.Mesh`) _output)
    (bind _returnvalue (`AnimSequenceBase.GetPlayLength` _output))
    (`KismetSystemLibrary.Delay` _returnvalue)
    (set `self.isTaunt` false)
    (`self.ChasePlayer`)
    (else
      (`self.ChasePlayer`))))

(event `Multi_PlayerMontague`
  (params (InSkeletalMeshComponent :type "SkeletalMeshComponent Object Reference") (MontageToPlay :type "AnimMontage Object Reference") (StartingSection :type Name))
  ;[1 1 1] Aggro
  (`|PlayMontage` InSkeletalMeshComponent MontageToPlay 1.0 0.0 StartingSection))

(event `self.ChasePlayer`
  ;[1 1 1] Aggro
  ;;[1 1 1] Chasing
  (if (`self.isCombat`)
    (`|AIMoveTo` self (0.0 0.0 0.0) (`self.PlayerTarget`) 50.0
      (:`OnSuccess`
        (`self.RunAttackChoice`))
      (:`OnFail`
        (`KismetSystemLibrary.PrintString` "Fail" true true (struct :`R` 1.0 :`G` 0.061921 :`A` 1.0) 5.0)
        (`self.ClearTarget`)))))

(event `self.RunAttackChoice`
  (bind _playertarget (`self.PlayerTarget`)
    (:`then`
      (bind _dead (message `/Game/_Main/Interfaces/INT_HeroCharacter.isDead` _playertarget))
      (if (not _dead)
        (bind _length (`self.f_PickAttack` (`self.GetDistanceTo` self (`self.PlayerTarget`))))
        (`KismetSystemLibrary.Delay` (+ _length 0.5))
        (`self.ChasePlayer`)
        (else
          (`self.ClearTarget`))))
    (:`else`
      (`self.ClearTarget`))))

(event `self.ClearTarget`
  ;[1 0 0.03689] To Do
)

(event `self.SetMeleeCollision`
  (params (State :type Boolean))
  (if State
    (`PrimitiveComponent.SetCollisionEnabled` (`self.MeleeSphere`) "QueryOnly")
    (else
      (`PrimitiveComponent.SetCollisionEnabled` (`self.MeleeSphere`) "NoCollision"))))

(event `self.MeleeSphere.OnComponentBeginOverlap`
  (params (OverlappedComponent :type "PrimitiveComponent Object Reference") (OtherActor :type "Actor Object Reference") (OtherComp :type "PrimitiveComponent Object Reference") (OtherBodyIndex :type Integer) (bFromSweep :type Boolean) (SweepResult :type "HitResult Structure (by ref)"))
  (`/Engine/EditorBlueprintResources/ActorMacros.Switch Has Authority`
    (:`Authority`
      (if (`self.ActorHasTag` OtherActor "Player")
        (`self.f_GetDamage` OtherActor)))))

(event `self.DoSphereOverlap`
  (`/Engine/EditorBlueprintResources/ActorMacros.Switch Has Authority`
    (:`Authority`
      (bind _outactors (`KismetSystemLibrary.SphereOverlapActors` (+ (`self.K2_GetActorLocation`) (* (`self.GetActorForwardVector`) 200.0)) 100.0 (`|MakeArray` "ObjectTypeQuery3" :!type "EObjectTypeQuery Enum") null (`|MakeArray` self :!type "Actor Object Reference")))
      (for _array_element _outactors
        (if (`self.ActorHasTag` _array_element "Player")
          (`self.f_GetDamage` _array_element))))))

(event `self.DoRangeAttack`)

(fn `f_GetAttackType`
  (returns (AttackType :type "/Game/_Main/AI/E_AIAttackTypes Enum"))
  (return (`self.AttackType`)))

(fn `f_GetCombatState`
  (returns (isCombat :type Boolean))
  (return (`self.isCombat`)))

(fn `f_GetDamage`
  (params (`Hit Player` :type "Actor Object Reference"))
  (switch `/Game/_Main/AI/E_AIAttackTypes` (`self.AttackType`)
    (:`NewEnumerator0`
      (`GameplayStatics.ApplyDamage` `Hit Player` (`self.LightAttackDamage`) null self "/Script/Engine.DamageType"))
    (:`NewEnumerator1`
      (`GameplayStatics.ApplyDamage` `Hit Player` (`self.HeavyAttackDamage`) null self "/Script/Engine.DamageType"))
    (:`NewEnumerator2`
      (`GameplayStatics.ApplyDamage` `Hit Player` (`self.RangeAttackDamage`) null self "/Script/Engine.DamageType"))
    (:`NewEnumerator3`
      (`GameplayStatics.ApplyDamage` `Hit Player` (`self.SpecialAttackDamage`) null self "/Script/Engine.DamageType"))))

(fn `f_GetMontage`
  (params (Montage :type "Array of AnimMontage Object Reference"))
  (returns (Output :type "AnimMontage Object Reference"))
  (return (`|GetArrayItem` Montage (`KismetMathLibrary.RandomIntegerInRange` 0 (- (`KismetArrayLibrary.Array_Length` Montage) 1)))))

(fn `f_GetPlayerTarget`
  (returns (PlayerTarget :type "Actor Object Reference"))
  (return (`self.PlayerTarget`)))

(fn `f_MovementState`
  (params (State :type "/Game/_Main/AI/E_AIMovementState Enum" :default "NewEnumerator0"))
  (bind _walkspeed (`self.WalkSpeed`))
  (set `CharacterMovementComponent.MaxWalkSpeed` (select `/Game/_Main/AI/E_AIMovementState` State :`NewEnumerator1` _walkspeed :`NewEnumerator2` (* (`self.SpeedMultiplier`) _walkspeed)) (`self.CharacterMovement`)))

(fn `f_Percentage`
  (params (Percent :type "Float (double-precision)"))
  (returns (Return :type Boolean))
  (return (select `bool` (== Percent 0.0) :`false` (<= (`KismetMathLibrary.RandomFloatInRange` 0.0 100.0) Percent))))

(fn `f_PickAttack`
  (params (DistanceToPlayer :type "Float (double-precision)"))
  (returns (Length :type "Float (double-precision)"))
  (bind _output (`self.f_GetMontage` (`self.SpecialAttackMontages`)))
  (bind _output_2 (`self.f_GetMontage` (`self.LightAttackMontages`)))
  (bind _output_3 (`self.f_GetMontage` (`self.RangeAttackMontages`)))
  (bind _output_4 (`self.f_GetMontage` (`self.HeavytAttackMontages`)))
  (if (<= DistanceToPlayer (`self.Melee Distance`))
    (if (`self.f_Percentage` 70.0)
      (set `self.AttackType` "NewEnumerator0")
      (`self.Multi_PlayerMontague` (`self.Mesh`) _output_2)
      (bind _returnvalue (`AnimSequenceBase.GetPlayLength` _output_2))
      (return _returnvalue)
      (else
        (set `self.AttackType` "NewEnumerator1")
        (`self.Multi_PlayerMontague` (`self.Mesh`) _output_4)
        (bind _returnvalue_2 (`AnimSequenceBase.GetPlayLength` _output_4))
        (return _returnvalue_2)))
    (elif (<= DistanceToPlayer (`self.RangeDistance`))
      (set `self.AttackType` "NewEnumerator3")
      (`self.Multi_PlayerMontague` (`self.Mesh`) _output)
      (bind _returnvalue_3 (`AnimSequenceBase.GetPlayLength` _output))
      (return _returnvalue_3)
      (else
        (set `self.AttackType` "NewEnumerator2")
        (`self.Multi_PlayerMontague` (`self.Mesh`) _output_3)
        (bind _returnvalue_4 (`AnimSequenceBase.GetPlayLength` _output_3))
        (return _returnvalue_4)))))

(fn `OnRep_isTaunt`
  (if (`self.isTaunt`)
    (`GameplayStatics.PlaySoundAtLocation` (`self.TauntSound`) (`self.K2_GetActorLocation` self) (struct) 1.0 1.0 0.0 null null null)))

(fn `UserConstructionScript`
  (`parent.UserConstructionScript`))